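; World game mode that drives a periodic hunger update for the animals in the level.
; BeginPlay caches all BP_Animal actors once, so animals spawned later are not included.
; Tick accumulates delta time and, roughly every two seconds, fires CallHunger on the cached animals and resets the timer.
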(event `self.ReceiveBeginPlay`
  (bind _outactors (`GameplayStatics.GetAllActorsOfClass` "/Game/Blueprints/Actors/BP_Animal.BP_Animal_C"))
  (set `self.Actors` _outactors))

(event `self.ReceiveTick`
  (params (DeltaSeconds :type "Float (single-precision)"))
  (bind _output_get (set `self.timer_Hunger` (+ DeltaSeconds (`self.timer_Hunger`))))
  (if (> _output_get 2.0)
    (`/Game/Blueprints/Actors/BP_Animal.call_Hunger` (`self.Actors`))
    (set `self.timer_Hunger` 0.0)))

(fn `UserConstructionScript`)