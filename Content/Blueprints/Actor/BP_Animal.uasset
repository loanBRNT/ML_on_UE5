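; BP_Animal is an animal actor that tracks Hunger, Stamina and Health and shows each value on its own text element.
; BeginPlay fills the three texts and binds the tick_hunger event to CallHunger, which lowers Hunger by one while the animal is Hungry and Hunger is above zero.
; Each stat has a Maj update function that adds a signed value and refreshes its text, though only the hunger one is called here.
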(event `self.ReceiveBeginPlay`
  (`TextRenderComponent.K2_SetText` (`self.Hunger_text`) (`KismetTextLibrary.Conv_IntToText` (`self.hunger`)))
  (`TextRenderComponent.K2_SetText` (`self.Stamina_text`) (`KismetTextLibrary.Conv_IntToText` (`self.stamina`)))
  (`TextRenderComponent.K2_SetText` (`self.Health_text`) (`KismetTextLibrary.Conv_IntToText` (`self.health`)))
  (add `self.call_Hunger` (delegate `tick_hunger`)))

(event `self.ReceiveTick`
  (params (DeltaSeconds :type "Float (single-precision)")))

(event `tick_hunger`
  (if (and (> (`self.hunger`) 0) (`self.hungry`))
    (`self.majHunger` -1)))

(fn `majHealth`
  (params (Valeur :type Integer))
  (bind _output_get (set `self.health` (+ (`self.health`) Valeur)))
  (`TextRenderComponent.K2_SetText` (`self.Health_text`) (`KismetTextLibrary.Conv_IntToText` _output_get)))

(fn `majHunger`
  (params (Valeur :type Integer))
  (bind _output_get (set `self.hunger` (+ (`self.hunger`) Valeur)))
  (`TextRenderComponent.K2_SetText` (`self.Hunger_text`) (`KismetTextLibrary.Conv_IntToText` _output_get)))

(fn `majStamina`
  (params (Valeur :type Integer))
  (bind _output_get (set `self.stamina` (+ (`self.stamina`) Valeur)))
  (`TextRenderComponent.K2_SetText` (`self.Stamina_text`) (`KismetTextLibrary.Conv_IntToText` _output_get)))

(fn `UserConstructionScript`)