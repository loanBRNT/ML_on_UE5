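; AI controller for animals that tracks food sources and hunger for the animal's AI through its Blackboard.
; AI Perception updates on actors tagged "Plants" store the plant's location as the food position and set SeeFood, or clear that flag when sensing is lost.
; MajBBLookForFood writes the Hungry flag from its input and prints the value to screen.
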(event `self.AIPerception.OnTargetPerceptionUpdated`
  (params (Actor :type "Actor Object Reference") (Stimulus :type "AIStimulus Structure"))
  (bind _blackboard (`self.Blackboard`))
  (if (`self.ActorHasTag` Actor "Plants")
    (if (`.bSuccessfullySensed` (break `AIStimulus` Stimulus))
      (`BlackboardComponent.SetValueAsVector` _blackboard "Food Position" (`self.K2_GetActorLocation` Actor))
      (`BlackboardComponent.SetValueAsBool` _blackboard "SeeFood" true)
      (else
        (`BlackboardComponent.SetValueAsBool` _blackboard "SeeFood" false)))))

(fn `majBBLookForFood`
  (params (BoolValue :type Boolean))
  (`KismetSystemLibrary.PrintString` (`KismetStringLibrary.Conv_BoolToString` BoolValue))
  (`BlackboardComponent.SetValueAsBool` (`self.Blackboard`) "Hungry" BoolValue))

(fn `UserConstructionScript`)