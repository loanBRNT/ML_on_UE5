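; Animal actor for an ecosystem simulation, with hunger, stamina and death, driven alongside an AI_Animal controller.
; A bound hunger tick handles rest and sprint stamina, counts down satiety, drains hunger, flags food search on the AI blackboard and kills the animal at zero.
; Eating refills hunger and kills animal prey or destroys plants, reporting deaths and plant losses to GameModeWorld.
; Text components display the stats.
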(event `self.ReceiveBeginPlay`
  (bind _asai_animal (cast `/Game/Blueprints/AI/AI_Animal` (`AIBlueprintHelperLibrary.GetAIController` self)))
  (set `self.As AI Animal` _asai_animal)
  (add `self.call_Hunger` (delegate `tick_hunger`)))

(event `tick_hunger`
  (if (`self.resting`)
    (if (>= (`self.stamina`) 50)
      (set `self.resting` false)
      (else
        (`self.majStamina` 2)
        (if (`self.sprint`) :!label _label
          (`self.majStamina` -2)
          (if (<= (`self.stamina`) 0)
            (set `self.tired` true)))
        (if (> (`self.hunger`) 0)
          (if (`self.hungry`)
            (`self.majHunger` -1)
            (if (and (<= (`self.hunger`) 75) (not (`self.lookForFood`)))
              (`/Game/Blueprints/AI/AI_Animal.majBBLookForFood` (`self.As AI Animal`) true)
              (set `self.lookForFood` true))
            (else
              (bind _result (`/Engine/EditorBlueprintResources/StandardMacros.DecrementInt` (`self.repus`))
                (:`  `
                  (if (<= _result 0)
                    (set `self.hungry` true))))))
          (else
            (`self.mourir`)))))
    (else
      (goto _label))))

(event `start resting`
  (set `self.resting` true))

(event `self.manger`
  (params (ActorEaten :type "Actor Object Reference"))
  (if (`self.hungry`)
    (set `self.repus` 5)
    (set `self.hungry` false)
    (set `self.lookForFood` false)
    (`/Game/Blueprints/AI/AI_Animal.majBBLookForFood` (`self.As AI Animal`) false)
    (bind _asbp_animal (cast `/Game/Blueprints/Actors/BP_Animal` ActorEaten)
      (:`then`
        (`self.mourir` _asbp_animal))
      (:`CastFailed`
        (`self.K2_DestroyActor` ActorEaten)
        (bind _asgame_mode_world (cast `/Game/Blueprints/Game/GameModeWorld` (`GameplayStatics.GetGameMode`)))
        (`/Game/Blueprints/Game/GameModeWorld.update plants` _asgame_mode_world -1)))
    (`self.majHunger` 100)))

(event `self.mourir`
  (bind _asgame_mode_world (cast `/Game/Blueprints/Game/GameModeWorld` (`GameplayStatics.GetGameMode`)))
  (`/Game/Blueprints/Game/GameModeWorld.dead animal list` _asgame_mode_world self)
  (`self.K2_DestroyActor`))

(fn `getEpuise`
  (returns (epuise :type Boolean))
  (return (`self.tired`)))

(fn `isResting`
  (returns (resting :type Boolean))
  (return (`self.resting`)))

(fn `majHealth`
  (params (Valeur :type Integer))
  (bind _output_get (set `self.breed` (+ (`self.breed`) Valeur)))
  (`TextRenderComponent.K2_SetText` (`self.Health_text`) (`KismetTextLibrary.Conv_IntToText` _output_get)))

(fn `majHunger`
  (params (Valeur :type Integer))
  (bind _output_get (set `self.hunger` (+ (`self.hunger`) Valeur)))
  (if (not (<= _output_get 100))
    (set `self.hunger` 100))
  (`TextRenderComponent.K2_SetText` (`self.Hunger_text`) (`KismetTextLibrary.Conv_IntToText` (`self.hunger`))))

(fn `majStamina`
  (params (Valeur :type Integer))
  (bind _output_get (set `self.stamina` (+ (`self.stamina`) Valeur)))
  (`TextRenderComponent.K2_SetText` (`self.Stamina_text`) (`KismetTextLibrary.Conv_IntToText` _output_get)))

(fn `setSprint`
  (params (sprint :type Boolean))
  (set `self.sprint` sprint))

(fn `UserConstructionScript`
  (`TextRenderComponent.K2_SetText` (`self.Hunger_text`) (`KismetTextLibrary.Conv_IntToText` (`self.hunger`)))
  (`TextRenderComponent.K2_SetText` (`self.Stamina_text`) (`KismetTextLibrary.Conv_IntToText` (`self.stamina`)))
  (`TextRenderComponent.K2_SetText` (`self.Health_text`) (`KismetTextLibrary.Conv_IntToText` (`self.breed`))))